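; GameplayCharacter_BP is a character Blueprint that switches its over-the-shoulder camera between a normal and an aiming view.
; Every Tick polls IsAiming and, while it is true, SetCamPos narrows the FollowCam field of view and raises the Boom socket offset.
; Otherwise Tick restores the default offset, arm length and field of view, snapping between views without interpolation.
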(event EventTick
  (params (DeltaSeconds :type Float%20%28single-precision%29))
  (bind _boom (Variables|Default|GetBoom))
  (if (Variables|Default|GetIsAiming)
    (CallFunction|SetCamPos)
    (else
      (Variables|/Script/Engine.SpringArmComponent|SetSocketOffset _boom "0,60.000000,25.000000")
      (Variables|/Script/Engine.SpringArmComponent|SetTargetArmLength _boom 1.5e+02)
      (Camera|SetFieldOfView (Variables|Default|GetFollowCam) 9e+01))))

(fn ConstructionScript)

(fn SetCamPos
  (if (Variables|Default|GetIsAiming)
    (Camera|SetFieldOfView (Variables|Default|GetFollowCam) 6e+01)
    (Variables|/Script/Engine.SpringArmComponent|SetSocketOffset (Variables|Default|GetBoom) "0,60.000000,75.000000")))