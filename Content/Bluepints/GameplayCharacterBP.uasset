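; Player character Blueprint that handles aim-down-sights camera framing and switching between two weapons.
; Every Tick, it reads IsAiming, which is not set here, to snap boom length, socket offset and first-person camera FOV between aim and default values.
; Pressing Q flips IsHoldingRifle, swapping the Rifle and SK_FPGun meshes between WeaponHolder and WeaponSocket and shifting the holder's position.
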(event EventBeginPlay
  (Variables|Default|SetIsHoldingRifle true))

(event EventTick
  (params (DeltaSeconds :type Float%20%28single-precision%29))
  (CallFunction|SettingCamforADS))

(event Input|KeyboardEvents|Q
  (params (Key :type Key%20Structure))
  (:Pressed
    (CallFunction|WeaponSwitch)))

(fn ConstructionScript)

(fn SettingCamforADS
  (bind _boom (Variables|Default|Getboom))
  (bind _boom_2 (Variables|Default|Getboom))
  (if (Variables|Default|GetIsAiming)
    (Variables|/Script/Engine.SpringArmComponent|SetTargetArmLength _boom 1e+02)
    (Variables|/Script/Engine.SpringArmComponent|SetSocketOffset _boom "0,50.000000,30.000000")
    (Camera|SetFieldOfView (Variables|Default|GetFPCam) 6e+01)
    (else
      (Variables|/Script/Engine.SpringArmComponent|SetTargetArmLength _boom_2 1.5e+02)
      (Variables|/Script/Engine.SpringArmComponent|SetSocketOffset _boom_2 "0,60.000000,15.000000")
      (Camera|SetFieldOfView (Variables|Default|GetFPCam) 9e+01))))

(fn WeaponSwitch
  (bind _weaponholder (Variables|Default|GetWeaponHolder))
  (bind _weaponholder_2 (Variables|Default|GetWeaponHolder))
  (if (Variables|Default|GetIsHoldingRifle)
    (Class|SkinnedMeshComponent|SetSkeletalMesh _weaponholder_2 "/Game/Weapons/Rifle.Rifle" true)
    (Transformation|SetRelativeLocation _weaponholder_2 "0,10.000000, 0" false false)
    (Class|SkinnedMeshComponent|SetSkeletalMesh (Variables|Default|GetWeaponSocket) "/Game/FirstPerson/FPWeapon/Mesh/SK_FPGun.SK_FPGun" true)
    (Variables|Default|SetIsHoldingRifle false)
    (else
      (Class|SkinnedMeshComponent|SetSkeletalMesh _weaponholder "/Game/FirstPerson/FPWeapon/Mesh/SK_FPGun.SK_FPGun" true)
      (Transformation|SetRelativeLocation _weaponholder "0,20.000000, 0" false false)
      (Class|SkinnedMeshComponent|SetSkeletalMesh (Variables|Default|GetWeaponSocket) "/Game/Weapons/Rifle.Rifle" true)
      (Variables|Default|SetIsHoldingRifle true))))